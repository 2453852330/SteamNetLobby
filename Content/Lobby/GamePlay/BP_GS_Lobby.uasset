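; Lobby GameState that holds the list of player infos and their ready states for the pre-game lobby.
; The first player added is recorded as host; players are toggled or removed by name through library helpers.
; The list's RepNotify messages player controller 0 through an interface to refresh the player list UI.
; A check reports whether every listed player is ready to start play.
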(fn `AddPlayerInfoToList`
  (params (PlayerInfo :type "LobbyPlayerInfo Structure (by ref)"))
  (if (== (`KismetArrayLibrary.Array_Length` (`self.PlayerInfoList`)) 0)
    (set `self.HostName` (`.PlayerName` (break `LobbyPlayerInfo` PlayerInfo))))
  (`KismetArrayLibrary.Array_Add` (`self.PlayerInfoList`) PlayerInfo))

(fn `CheckIsAllReadyToStartPlay`
  (returns (`Is Ready` :type Boolean))
  (for _array_element (`self.PlayerInfoList`)
    (if (not (`.bIsReady` (break `LobbyPlayerInfo` _array_element)))
      (return false)))
  (return true))

(fn `OnRep_PlayerInfoList`
  (message `/SteamNetLobby/Lobby/BP/BPI_PC_Interface.BPI_UpdatePlayerListUI` (`GameplayStatics.GetPlayerController` 0)))

(fn `RemovePlayer`
  (params (PlayerName :type Text))
  (`LibLobbyHelper.LibRemovePlayerByName` (`self.PlayerInfoList`) PlayerName))

(fn `UpdatePlayerReadyState`
  (params (PlayerName :type Text))
  (`LibLobbyHelper.LibUpdatePlayerReadyState` (`self.PlayerInfoList`) PlayerName))

(fn `UserConstructionScript`)