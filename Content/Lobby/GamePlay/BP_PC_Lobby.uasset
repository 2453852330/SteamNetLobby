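; Lobby player controller that creates the lobby UI and handles player registration, readiness, kicking and match start.
; A client RPC sends the Steam name to BP_GS_Lobby via a server RPC, while a looping timer polls to refresh the player list.
; Interface events drive the ready toggle, kick and all-ready-gated server travel.
; Kicks broadcast to every controller, and the matching name destroys its session and returns to the main menu.
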(event `LetClientUpdatePlayerName_Client`
  ;[1 0.9844 0] On Post Login To Add Player Info to GameState
  (bind _output_get (set `self.PlayerName_Client` (`KismetTextLibrary.Conv_StringToText` (`KKSessionSubsystem.KKGetSteamPlayerName` (subsystem `KKSessionSubsystem`) self))))
  (`self.AddPlayerToServerPlayerList_Server` (make `LobbyPlayerInfo` _output_get)))

(event `AddPlayerToServerPlayerList_Server`
  (params (PlayerInfo :type "LobbyPlayerInfo Structure"))
  ;[1 0.9844 0] On Post Login To Add Player Info to GameState
  (bind _asbp_gs_lobby (cast `/SteamNetLobby/Lobby/GamePlay/BP_GS_Lobby` (`GameplayStatics.GetGameState`)))
  (`/SteamNetLobby/Lobby/GamePlay/BP_GS_Lobby.AddPlayerInfoToList` _asbp_gs_lobby PlayerInfo))

(event `self.ReceiveBeginPlay`
  ;[1 0.1406 0] begin
  (if (`self.IsLocalPlayerController`)
    (set `self.bShowMouseCursor` true)
    (bind _returnvalue (`|CreateWidget` "/SteamNetLobby/Lobby/UI/UI_Lobby.UI_Lobby_C" self))
    (bind _output_get (set `self.UI_Lobby` _returnvalue))
    (`UserWidget.AddToViewport` _output_get 0)
    ;[0 0.6484 1] timer to auto refresh server ui , this is the simplest way to show server ui
    (`KismetSystemLibrary.K2_SetTimerDelegate` (`|CreateDelegate` :!event `Timer_OnAutoUpdatePlayerListUI`) 0.5 true)))

(event `Timer_OnAutoUpdatePlayerListUI`
  ;[0 0.6484 1] timer to auto refresh server ui , this is the simplest way to show server ui
  (bind _ui_lobby (`self.UI_Lobby`)
    (:`then`
      (`/SteamNetLobby/Lobby/UI/UI_Lobby.UpdatePlayer` _ui_lobby))
    (:`else`)))

(event `/SteamNetLobby/Lobby/BP/BPI_PC_Interface.BPI_UpdatePlayerListUI`
  ;[1 0 0.5625] interface : update player ui
  (bind _ui_lobby (`self.UI_Lobby`)
    (:`then`
      (`/SteamNetLobby/Lobby/UI/UI_Lobby.UpdatePlayer` _ui_lobby))
    (:`else`)))

(event `/SteamNetLobby/Lobby/BP/BPI_PC_Interface.BPI_UpdateReadyState`
  ;[0.9688 1 0] interface + rpc : update ready state
  (`self.UpdatePlayerReadyState_Server` (`self.PlayerName_Client`)))

(event `UpdatePlayerReadyState_Server`
  (params (PlayerName :type Text))
  ;[0.9688 1 0] interface + rpc : update ready state
  (bind _asbp_gs_lobby (cast `/SteamNetLobby/Lobby/GamePlay/BP_GS_Lobby` (`GameplayStatics.GetGameState`)))
  (`/SteamNetLobby/Lobby/GamePlay/BP_GS_Lobby.UpdatePlayerReadyState` _asbp_gs_lobby PlayerName))

(event `/SteamNetLobby/Lobby/BP/BPI_PC_Interface.BPI_KickPlayer`
  (params (PlayerName :type Text))
  ;[0.9453 0 1] interface + RPC : kick player
  (bind _asbp_gs_lobby (cast `/SteamNetLobby/Lobby/GamePlay/BP_GS_Lobby` (`GameplayStatics.GetGameState`)))
  (`/SteamNetLobby/Lobby/GamePlay/BP_GS_Lobby.RemovePlayer` _asbp_gs_lobby PlayerName)
  (bind _outactors (`GameplayStatics.GetAllActorsOfClass` "BP_PC_Lobby_C"))
  (for _array_element _outactors
    (`self.CheckNameToKick_Client` _array_element PlayerName) ; NOTE: Target is the find player controllers
  ))

(event `CheckNameToKick_Client`
  (params (Name :type Text))
  ;[0.9453 0 1] interface + RPC : kick player
  (if (`KismetTextLibrary.EqualEqual_TextText` Name (`self.PlayerName_Client`))
    (`KKSessionSubsystem.KKDestorySession` (subsystem `KKSessionSubsystem`) self)
    (`/SteamNetLobby/Lobby/Lib/BPL_Lobby.BPL_ShowBlur` self)
    (`/SteamNetLobby/Lobby/Lib/BPL_Lobby.BPL_ShowMsg` self "You have been kicked out")
    (`KismetSystemLibrary.Delay` 3.0)
    (`GameplayStatics.OpenLevelBySoftObjectPtr` "/SteamNetLobby/Lobby/Maps/Map_MainMenu.Map_MainMenu") ; i dont handle destory bind in c++, so need to handle in here when the session is destoryed
  ))

(event `/SteamNetLobby/Lobby/BP/BPI_PC_Interface.BPI_ServerTravel`
  ;[0.9453 0 1] interface + RPC : Server Travel
  (bind _asbp_gs_lobby (cast `/SteamNetLobby/Lobby/GamePlay/BP_GS_Lobby` (`GameplayStatics.GetGameState`)))
  (if (`/SteamNetLobby/Lobby/GamePlay/BP_GS_Lobby.CheckIsAllReadyToStartPlay` _asbp_gs_lobby)
    (`|ExecutionSequence`
      (:`then_0`
        (bind _outactors (`GameplayStatics.GetAllActorsOfClass` "BP_PC_Lobby_C"))
        (for _array_element _outactors
          (`self.ShowLoadUI_Client` _array_element)))
      (:`then_1`
        (`LibLobbyHelper.LibServerTravel` self "/SteamNetLobby/Lobby/Maps/Map_Game_LobbyTest.Map_Game_LobbyTest")))
    (else
      (`/SteamNetLobby/Lobby/Lib/BPL_Lobby.BPL_ShowMsg` self "Players Is Not Ready"))))

(event `ShowLoadUI_Client`
  ;[0.9453 0 1] interface + RPC : Server Travel
  (`/SteamNetLobby/Lobby/Lib/BPL_Lobby.BPL_ShowLoadMapUI` self))

(fn `UserConstructionScript`)